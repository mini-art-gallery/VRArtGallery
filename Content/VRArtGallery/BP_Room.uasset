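; BP_Room is a resizable room actor for the VR art gallery, built from four walls, a floor and a ceiling.
; Its construction script passes Width, Length and Height as a scale vector to SetGlobalScale for each mesh.
; SetGlobalScale multiplies the mesh's relative transform matrix by a scale matrix, so positions and rotated pieces scale along the room's axes.
; The event graph has no active logic.
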(event EventBeginPlay)

(event Collision|EventActorBeginOverlap
  (params (OtherActor :type Actor%20Object%20Reference)))

(event EventTick
  (params (DeltaSeconds :type Float%20%28single-precision%29)))

(fn ConstructionScript
  (bind _width (Variables|Default|GetWidth))
  (bind _length (Variables|Default|GetLength))
  (bind _height (Variables|Default|GetHeight))
  (bind _returnvalue (Math|Vector|MakeVector _width _length _height))
  (CallFunction|SetGlobalScale (Variables|Default|GetFrontWall) _returnvalue)
  (CallFunction|SetGlobalScale (Variables|Default|GetFloorMesh) _returnvalue)
  (CallFunction|SetGlobalScale (Variables|Default|GetCeilingMesh) _returnvalue)
  (CallFunction|SetGlobalScale (Variables|Default|GetBackWall) _returnvalue)
  (CallFunction|SetGlobalScale (Variables|Default|GetLeftWall) _returnvalue)
  (CallFunction|SetGlobalScale (Variables|Default|GetRightWall) _returnvalue))

(fn SetGlobalScale
  (params (Mesh :type Scene%20Component%20Object%20Reference) (Scale :type Vector))
  (Transformation|SetRelativeTransform Mesh (Math|Conversions|ToTransform(Vector) (* (Math|Transform|ToMatrix(Transform) (Transformation|GetRelativeTransform Mesh)) (Math|Transform|ToMatrix(Transform) (Math|Transform|MakeTransform "0, 0, 0" "0, 0, 0" Scale)))) false false))