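; BP_Room is a parametric room actor built from floor, ceiling and four wall meshes, sized by Width, Length and Height.
; Its construction script scales every mesh from those dimensions, with the left and right walls using half Height vertically.
; Only the front and back walls are repositioned, offset along X by half the width and raised to half height at 100 units per size unit.
; The event graph holds no active logic.
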(event EventBeginPlay)

(event Collision|EventActorBeginOverlap
  (params (OtherActor :type Actor%20Object%20Reference)))

(event EventTick
  (params (DeltaSeconds :type Float%20%28single-precision%29)))

(fn ConstructionScript
  (bind _length (Variables|Default|GetLength))
  (bind _width (Variables|Default|GetWidth))
  (bind _height (Variables|Default|GetHeight))
  (bind _frontwall (Variables|Default|GetFrontWall))
  (bind _backwall (Variables|Default|GetBackWall))
  (bind _height_2 (Variables|Default|GetHeight))
  (bind _length_2 (Variables|Default|GetLength))
  (bind _width_2 (Variables|Default|GetWidth))
  (bind _returnvalue (/ _width_2 1.0))
  (bind _returnvalue_2 (/ _length 1.0))
  (bind _returnvalue_3 (/ _width 1.0))
  (bind _returnvalue_4 (/ _height 1.0))
  (bind _returnvalue_5 (/ _length_2 1.0))
  (bind _returnvalue_6 (/ _height_2 2.0))
  (bind _returnvalue_7 (Math|Vector|MakeVector _returnvalue_5 1.0 _returnvalue_6))
  (bind _returnvalue_8 (Math|Vector|MakeVector _returnvalue _returnvalue_2 1.0))
  (bind _returnvalue_9 (Math|Vector|MakeVector _returnvalue_3 1.0 _returnvalue_4))
  (Transformation|SetRelativeScale3D (Variables|Default|GetCeilingMesh) _returnvalue_8)
  (Transformation|SetRelativeScale3D (Variables|Default|GetFloorMesh) _returnvalue_8)
  (Transformation|SetRelativeScale3D _frontwall _returnvalue_9)
  (Transformation|SetRelativeScale3D _backwall _returnvalue_9)
  (Transformation|SetRelativeScale3D (Variables|Default|GetLeftWall) _returnvalue_7)
  (Transformation|SetRelativeScale3D (Variables|Default|GetRightWall) _returnvalue_7)
  (Transformation|SetRelativeLocation _frontwall (Math|Vector|MakeVector (/ (* (Variables|Default|GetWidth) -1e+02) 2.0) 0.0 (/ (* (Variables|Default|GetHeight) 1e+02) 2.0)) false false)
  (Transformation|SetRelativeLocation _backwall (Math|Vector|MakeVector (/ (* (Variables|Default|GetWidth) 1e+02) 2.0) 0.0 (/ (* (Variables|Default|GetHeight) 1e+02) 2.0)) false false))